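; Spawner that procedurally builds a lane-crossing level from BP_Lane actors placed 100 units apart along Y.
; BeginPlay lays starter lanes, a highway and several random chunks, each lane receiving a reference back to the spawner.
; SpawnChunk adds grass, highway, water or track runs, never repeating the previous chunk type.
; At the active lane cap, it instead destroys the oldest lane if far enough behind the supplied Y position.
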(event EventBeginPlay
  (CallFunction|SpawnLane)
  (CallFunction|SpawnLane 1)
  (CallFunction|SpawnHighway)
  (for _index (range 0 5)
    (CallFunction|SpawnChunk)))

(event Collision|EventActorBeginOverlap
  (params (OtherActor :type Actor%20Object%20Reference)))

(event EventTick
  (params (DeltaSeconds :type Float%20%28single-precision%29)))

(fn ConstructionScript)

(fn SpawnLane
  (params (LaneType :type Integer))
  (bind _lanecount (Variables|Default|GetLaneCount))
  (bind _returnvalue (Game|SpawnActorfromClass "/Game/Blueprints/BP_Lane.BP_Lane_C" (Math|Transform|MakeTransform (Math|Vector|MakeVector 0.0 (Math|Conversions|ToFloat(Integer) (* _lanecount 100)) 0.0) "0, 0, 0" "1.000000,1.000000,1.000000") "Undefined" 0 0))
  (Default|SetType _returnvalue LaneType)
  (Variables|/Game/Blueprints/BP_Lane.BP_Lane_C|SetSpawner _returnvalue self)
  (Utilities|Map|Add (Variables|Default|GetLanes) _lanecount _returnvalue)
  (Math|Integer|IncrementInt _lanecount
    (:%20%20
      (Math|Integer|IncrementInt (Variables|Default|GetActiveLaneCount)
        (:%20%20
          (Default|Initialize _returnvalue))))))

(fn SpawnHighway
  (bind _returnvalue (Math|Random|RandomInteger 6))
  (Math|Integer|CompareInt _returnvalue
    (:>
      (for _index (range 0 _returnvalue)
        (CallFunction|SpawnLane 4)))
    (:==
      _))
  (CallFunction|SpawnLane 2))

(fn SpawnGrass
  (for _index (range 0 (Math|Random|RandomInteger 6))
    (Math|Integer|CompareInt (Math|Integer|%(Integer) _index 2)
      (:>
        (CallFunction|SpawnLane))
      (:==
        (CallFunction|SpawnLane 1)))))

(fn SpawnWater
  (for _index (range 0 (+ (Math|Random|RandomInteger 3) 2))
    (CallFunction|SpawnLane 5)))

(fn SpawnTracks
  (for _index (range 0 (+ (Math|Random|RandomInteger 6) 1))
    (CallFunction|SpawnLane 3)))

(fn SpawnChunk
  (params (Lane%20Y%20Position :type Integer))
  (bind _lanes (Variables|Default|GetLanes))
  (bind _lanesdeleted (Variables|Default|GetLanesDeleted))
  (bind (_value _returnvalue) (Utilities|Map|Find _lanes _lanesdeleted))
  (if (< (Variables|Default|GetActiveLaneCount) (Variables|Default|GetMaxLanes))
    (while (== (stale _output_get) (Variables|Default|GetLastLaneType))
      (bind _output_get (Variables|Default|SetCurrentLaneType (Math|Random|RandomInteger 4))))
    (switch int (Variables|Default|GetCurrentLaneType)
      (:0
        (CallFunction|SpawnGrass))
      (:1
        (CallFunction|SpawnHighway))
      (:2
        (CallFunction|SpawnWater))
      (:3
        (CallFunction|SpawnTracks)))
    (Variables|Default|SetLastLaneType (Variables|Default|GetCurrentLaneType))
    (elif _returnvalue
      (if (>= (- Lane%20Y%20Position (Math|Float|Truncate (.y (Transformation|GetActorLocation _value)))) 2000)
        (Actor|DestroyActor _value)
        (Utilities|Map|Remove _lanes _lanesdeleted)
        (Math|Integer|IncrementInt _lanesdeleted
          (:%20%20
            (Math|Integer|DecrementInt (Variables|Default|GetActiveLaneCount))))))))