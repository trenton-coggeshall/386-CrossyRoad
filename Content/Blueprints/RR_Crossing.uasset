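; Railroad crossing signal Blueprint that flashes a blue and an orange light alternately while it is activated.
; Tick counts down a short timer, and each time it expires flips a toggle that swaps full intensity between the two lights.
; DIsableLight clears the Activated flag and switches both lights off.
; Nothing in this Blueprint sets Activated to true.
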(event EventBeginPlay
  (Variables|Default|Setcountdown_timer 0.25)
  (Variables|Default|SetlightToggle false))

(event Collision|EventActorBeginOverlap
  (params (OtherActor :type Actor%20Object%20Reference)))

(event EventTick
  (params (DeltaSeconds :type Float%20%28single-precision%29))
  (if (Variables|Default|Getactivated)
    (Variables|Default|Setcountdown_timer (- (Variables|Default|Getcountdown_timer) DeltaSeconds))
    (Math|Float|CompareFloat (Variables|Default|Getcountdown_timer) 0.0
      (:<
        (bind _output_get (Variables|Default|SetlightToggle (not (Variables|Default|GetlightToggle))))
        (Variables|Default|Setcountdown_timer 0.25)
        (if _output_get
          (Rendering|Components|Light|SetIntensity (Variables|Default|GetBlueLight) 5e+03)
          (Rendering|Components|Light|SetIntensity (Variables|Default|GetOrangeLight) 0.0)
          (else
            (Rendering|Components|Light|SetIntensity (Variables|Default|GetBlueLight) 0.0)
            (Rendering|Components|Light|SetIntensity (Variables|Default|GetOrangeLight) 5e+03)))))))

(fn ConstructionScript)

(fn DIsableLight
  (Variables|Default|Setactivated false)
  (Rendering|Components|Light|SetIntensity (Variables|Default|GetOrangeLight) 0.0)
  (Rendering|Components|Light|SetIntensity (Variables|Default|GetBlueLight) 0.0))