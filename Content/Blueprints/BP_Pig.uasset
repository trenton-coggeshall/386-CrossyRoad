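; Player pig character that moves on two world axes, can be squashed or sunk, and shows a score widget on play.
; Axis input, gated by CanJump and CanMove, adds movement, snaps facing through RotatePlayer, and feeds a shared float comparison that gates Jump.
; SquashPig flattens the actor and SinkPig hides the mesh by zero scaling; both clear CanMove, after which pressing Jump reloads the level.
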(event EventBeginPlay
  (bind _returnvalue (UserInterface|CreateWidget "/Game/Blueprints/BP_Score.BP_Score_C"))
  (UserInterface|Viewport|AddtoViewport _returnvalue 0))

(event Collision|EventActorBeginOverlap
  (params (OtherActor :type Actor%20Object%20Reference)))

(event EventTick
  (params (DeltaSeconds :type Float%20%28single-precision%29)))

(event Input|ActionEvents|InputActionJump
  (params (Key :type Key%20Structure :default "None"))
  (:Pressed
    (if (not (Variables|Default|GetCanMove))
      (bind _returnvalue (Game|GetCurrentLevelName true))
      (Game|OpenLevel(byName) (Utilities|String|StringToName _returnvalue)))))

(event Input|AxisEvents|InputAxisUp-Down
  (params (AxisValue :type Float%20%28single-precision%29))
  (if (and (Character|CanJump) (Variables|Default|GetCanMove))
    (Pawn|Input|AddMovementInput "0.000000,1.000000,0.000000" AxisValue false)
    (CallFunction|RotatePlayer AxisValue 0.0)
    (Math|Float|CompareFloat AxisValue (stale Input|AxisEvents|InputAxisLeft-Right AxisValue)
      (:>
        _)
      (:<
        _))
    (Character|Jump)))

(event Input|AxisEvents|InputAxisLeft-Right
  (params (AxisValue :type Float%20%28single-precision%29))
  (if (and (Character|CanJump) (Variables|Default|GetCanMove))
    (Pawn|Input|AddMovementInput "1.000000,0.000000,0.000000" AxisValue false)
    (CallFunction|RotatePlayer 0.0 AxisValue)
    (Math|Float|CompareFloat (stale Input|AxisEvents|InputAxisUp-Down AxisValue) AxisValue
      (:>
        _)
      (:<
        _))
    (Character|Jump)))

(fn ConstructionScript)

(fn RotatePlayer
  (params (up-down :type Float%20%28double-precision%29) (left-right :type Float%20%28double-precision%29))
  (Math|Float|CompareFloat up-down 0.0
    (:>
      (Transformation|SetActorRotation "0.000000,90.000000,0.000000"))
    (:==
      (Math|Float|CompareFloat left-right 0.0
        (:>
          (Transformation|SetActorRotation "0, 0, 0"))
        (:<
          (Transformation|SetActorRotation "0.000000,180.000000,0.000000"))))
    (:<
      (Transformation|SetActorRotation "0.000000,-90.000000,0.000000"))))

(fn SquashPig
  (params (zsquash :type Boolean))
  (if (Variables|Default|GetCanMove)
    (if zsquash
      (Transformation|SetActorScale3D "0.500000,0.500000,0.100000")
      (else
        (Transformation|SetActorScale3D "0.500000,0.100000,0.500000")))
    (Variables|Default|SetCanMove false)))

(fn SinkPig
  (Transformation|SetWorldScale3D (Variables|Default|Getpig) "0, 0, 0")
  (Variables|Default|SetCanMove false))