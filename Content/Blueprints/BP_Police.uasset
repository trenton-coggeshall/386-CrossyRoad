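; BP_Police is a moving police car hazard that squashes BP_Pig actors it touches.
; Each tick it moves along world X by Speed, accumulates the distance traveled and destroys itself past a fixed limit in either direction.
; While active, it spins its blue and red lights through PoliceLights.
; Front and side box overlaps both call SquashPig on the pig, passing true for a front hit and false for a side hit.
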(event OnComponentBeginOverlap(FrontBox)
  (params (OverlappedComponent :type Primitive%20Component%20Object%20Reference) (OtherActor :type Actor%20Object%20Reference) (OtherComp :type Primitive%20Component%20Object%20Reference) (OtherBodyIndex :type Integer) (bFromSweep :type Boolean) (SweepResult :type Hit%20Result%20Structure%20%28by%20ref%29))
  (bind _asbp_pig (Utilities|Casting|CastToBP_Pig OtherActor))
  (Default|SquashPig _asbp_pig true))

(event OnComponentBeginOverlap(SideBox)
  (params (OverlappedComponent :type Primitive%20Component%20Object%20Reference) (OtherActor :type Actor%20Object%20Reference) (OtherComp :type Primitive%20Component%20Object%20Reference) (OtherBodyIndex :type Integer) (bFromSweep :type Boolean) (SweepResult :type Hit%20Result%20Structure%20%28by%20ref%29))
  (bind _asbp_pig (Utilities|Casting|CastToBP_Pig OtherActor))
  (Default|SquashPig _asbp_pig false))

(event EventBeginPlay)

(event Collision|EventActorBeginOverlap
  (params (OtherActor :type Actor%20Object%20Reference)))

(event EventTick
  (params (DeltaSeconds :type Float%20%28single-precision%29))
  (bind _returnvalue (Utilities|Time|GetWorldDeltaSeconds))
  (bind _speed (Variables|Default|GetSpeed))
  (bind _returnvalue_2 (* _speed _returnvalue))
  (Transformation|AddWorldOffset (Variables|Default|GetPoliceCar) (Math|Vector|MakeVector _returnvalue_2 0.0 0.0) false false)
  (bind _output_get (Variables|Default|SetDistanceTraveled (+ (Variables|Default|GetDistanceTraveled) _returnvalue_2)))
  (if (> (Math|Float|Absolute(Float) _output_get) 3.4e+03)
    (Actor|DestroyActor)
    (else
      (CallFunction|PoliceLights))))

(fn ConstructionScript)

(fn PoliceLights
  (bind _returnvalue (Utilities|Time|GetWorldDeltaSeconds))
  (bind _lightrotationspeed (Variables|Default|GetLightRotationSpeed))
  (bind _returnvalue_2 (* _lightrotationspeed _returnvalue))
  (Transformation|AddLocalRotation (Variables|Default|GetBlueLight) (Math|Rotator|MakeRotator 0.0 0.0 _returnvalue_2) false false)
  (Transformation|AddLocalRotation (Variables|Default|GetRedLight) (Math|Rotator|MakeRotator 0.0 0.0 _returnvalue_2) false false))