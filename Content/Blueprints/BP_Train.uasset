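; BP_Train is a train actor that travels in a straight line and removes itself after a set distance.
; Each Tick offsets the Caboose component along world X by Speed scaled by delta time and adds the same step to DistanceTravelled.
; Once that total passes a hard-coded limit, the actor destroys itself.
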(event EventBeginPlay)

(event Collision|EventActorBeginOverlap
  (params (OtherActor :type Actor%20Object%20Reference)))

(event EventTick
  (params (DeltaSeconds :type Float%20%28single-precision%29))
  (bind _returnvalue (Utilities|Time|GetWorldDeltaSeconds))
  (bind _speed (Variables|Default|GetSpeed))
  (bind _returnvalue_2 (* _speed _returnvalue))
  (Transformation|AddWorldOffset (Variables|Default|GetCaboose) (Math|Vector|MakeVector _returnvalue_2 0.0 0.0) false false)
  (bind _output_get (Variables|Default|SetDistanceTravelled (+ (Variables|Default|GetDistanceTravelled) _returnvalue_2)))
  (if (> _output_get 3.4e+03)
    (Actor|DestroyActor)))

(fn ConstructionScript)