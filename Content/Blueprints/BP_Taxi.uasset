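; BP_Taxi is a moving taxi hazard that squashes BP_Pig actors it runs into.
; Each tick it offsets the TaxiCar component along world X by Speed scaled by delta time, accumulating distance and destroying itself past a fixed absolute limit.
; Separate FrontBox and SideBox overlaps call SquashPig on the pig, with a boolean that distinguishes a front hit from a side hit.
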(event OnComponentBeginOverlap(SideBox)
  (params (OverlappedComponent :type Primitive%20Component%20Object%20Reference) (OtherActor :type Actor%20Object%20Reference) (OtherComp :type Primitive%20Component%20Object%20Reference) (OtherBodyIndex :type Integer) (bFromSweep :type Boolean) (SweepResult :type Hit%20Result%20Structure%20%28by%20ref%29))
  (bind _asbp_pig (Utilities|Casting|CastToBP_Pig OtherActor))
  (Default|SquashPig _asbp_pig false))

(event OnComponentBeginOverlap(FrontBox)
  (params (OverlappedComponent :type Primitive%20Component%20Object%20Reference) (OtherActor :type Actor%20Object%20Reference) (OtherComp :type Primitive%20Component%20Object%20Reference) (OtherBodyIndex :type Integer) (bFromSweep :type Boolean) (SweepResult :type Hit%20Result%20Structure%20%28by%20ref%29))
  (bind _asbp_pig (Utilities|Casting|CastToBP_Pig OtherActor))
  (Default|SquashPig _asbp_pig true))

(event EventBeginPlay)

(event Collision|EventActorBeginOverlap
  (params (OtherActor :type Actor%20Object%20Reference)))

(event EventTick
  (params (DeltaSeconds :type Float%20%28single-precision%29))
  (bind _returnvalue (Utilities|Time|GetWorldDeltaSeconds))
  (bind _speed (Variables|Default|GetSpeed))
  (bind _returnvalue_2 (* _speed _returnvalue))
  (Transformation|AddWorldOffset (Variables|Default|GetTaxiCar) (Math|Vector|MakeVector _returnvalue_2 0.0 0.0) false false)
  (bind _output_get (Variables|Default|SetDistanceTraveled (+ (Variables|Default|GetDistanceTraveled) _returnvalue_2)))
  (if (> (Math|Float|Absolute(Float) _output_get) 3.4e+03)
    (Actor|DestroyActor)))

(fn ConstructionScript)