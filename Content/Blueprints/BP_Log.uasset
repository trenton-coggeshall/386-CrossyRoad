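; BP_Log is a log actor that travels along the X axis and destroys itself once it has covered a fixed distance.
; Tick offsets the LogS mesh component by Speed scaled by delta time and adds the same step to DistanceTraveled for the despawn check.
; SetSize swaps that component's static mesh between small, medium and large log variants based on a size index.
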(event EventBeginPlay)

(event Collision|EventActorBeginOverlap
  (params (OtherActor :type Actor%20Object%20Reference)))

(event EventTick
  (params (DeltaSeconds :type Float%20%28single-precision%29))
  (bind _speed (Variables|Default|GetSpeed))
  (bind _returnvalue (* DeltaSeconds _speed))
  (Transformation|AddWorldOffset (Variables|Default|GetLogS) (Math|Vector|MakeVector _returnvalue 0.0 0.0) false false)
  (bind _output_get (Variables|Default|SetDistanceTraveled (+ _returnvalue (Variables|Default|GetDistanceTraveled))))
  (if (> _output_get 3.4e+03)
    (Actor|DestroyActor)))

(fn ConstructionScript)

(fn SetSize
  (params (Size :type Integer))
  (bind _logs (Variables|Default|GetLogS))
  (switch int Size
    (:0
      (Components|StaticMesh|SetStaticMesh _logs "/Game/Props/LogS.LogS"))
    (:1
      (Components|StaticMesh|SetStaticMesh _logs "/Game/Props/LogM.LogM"))
    (:2
      (Components|StaticMesh|SetStaticMesh _logs "/Game/Props/LogL.LogL"))))