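; BP_Lane is one lane in a Crossy Road-style game: grass, highway, railroad or water.
; SetType builds its tiles by LaneType, adding trees, obstacles and coins on grass, a rail crossing, or water with optional lily pads.
; Tick runs per-type timers spawning cars, trains with advance crossing warnings, or logs on water without lily pads.
; The first BP_Pig overlap increments LaneScore and asks Spawner for another chunk.
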(event OnComponentBeginOverlap(Box)
  (params (OverlappedComponent :type Primitive%20Component%20Object%20Reference) (OtherActor :type Actor%20Object%20Reference) (OtherComp :type Primitive%20Component%20Object%20Reference) (OtherBodyIndex :type Integer) (bFromSweep :type Boolean) (SweepResult :type Hit%20Result%20Structure%20%28by%20ref%29))
  (if (not (Variables|Default|GetLanePassed))
    (bind _asbp_pig (Utilities|Casting|CastToBP_Pig OtherActor))
    (Variables|/Game/Blueprints/BP_Pig.BP_Pig_C|SetLaneScore _asbp_pig (+ (Variables|/Game/Blueprints/BP_Pig.BP_Pig_C|GetLaneScore _asbp_pig) 1))
    (Default|SpawnChunk (Variables|Default|GetSpawner) (Math|Float|Truncate (.y (Transformation|GetActorLocation))))
    (Variables|Default|SetLanePassed true)))

(event EventBeginPlay)

(event Collision|EventActorBeginOverlap
  (params (OtherActor :type Actor%20Object%20Reference)))

(event EventTick
  (params (DeltaSeconds :type Float%20%28single-precision%29))
  (switch int (Variables|Default|GetLaneType)
    (:2
      (CallFunction|HighwayTick))
    (:3
      (CallFunction|RailroadTick))
    (:4
      (CallFunction|HighwayTick))
    (:5
      (CallFunction|WaterTick))))

(fn ConstructionScript)

(fn SetType
  (params (LaneType :type Integer))
  (bind _lanelength (Variables|Default|GetLaneLength))
  (bind _returnvalue (/ _lanelength 4))
  (bind _output_get (Variables|Default|SetLaneType LaneType))
  (if (< _output_get 4)
    (for _index (range 0 (Variables|Default|GetLaneLength))
      (bind _output_get_2 (Variables|Default|SetSpawnVector (Math|Vector|MakeVector (Math|Conversions|ToFloat(Integer) (* _index 80)) 0.0 0.0)))
      (bind _returnvalue_2 (AddComponent|AddStaticMeshComponent false (Math|Conversions|ToTransform(Vector) _output_get_2)))
      (switch int (Variables|Default|GetLaneType)
        (:0
          (Components|StaticMesh|SetStaticMesh _returnvalue_2 "/Game/Tiles/brightgrass.brightgrass")
          (if (or (>= _index (* _returnvalue 3)) (<= _index _returnvalue)) :!label _label
            (bind _returnvalue_3 (AddComponent|AddStaticMeshComponent false (Math|Transform|MakeTransform (Math|Vector|MakeVector (.x (Variables|Default|GetSpawnVector)) -2e+01 2e+01) "0, 0, 0" "1.000000,1.000000,1.000000")))
            (Components|StaticMesh|SetStaticMesh _returnvalue_3 "/Game/Props/SmallTree.SmallTree")
            (elif (<= (Math|Random|RandomFloat) 0.01)
              (Game|SpawnActorfromClass "/Game/Blueprints/BP_Coin.BP_Coin_C" (Math|Transform|MakeTransform (Math|Vector|MakeVector (.x (Variables|Default|GetSpawnVector)) (.y (Transformation|GetActorLocation)) 2e+01) "0, 0, 0" "1.000000,1.000000,1.000000") "Undefined" 0 0)
              (elif (<= (Math|Random|RandomFloat) 0.05)
                (bind _returnvalue_4 (AddComponent|AddStaticMeshComponent false (Math|Transform|MakeTransform (Math|Vector|MakeVector (.x (Variables|Default|GetSpawnVector)) 0.0 2e+01) "0, 0, 0" "1.000000,1.000000,1.000000")))
                (switch int (Math|Random|RandomInteger 3)
                  (:0
                    (Components|StaticMesh|SetStaticMesh _returnvalue_4 "/Game/Props/bush.bush"))
                  (:1
                    (Components|StaticMesh|SetStaticMesh _returnvalue_4 "/Game/Props/centerrock1.centerrock1"))
                  (:2
                    (Components|StaticMesh|SetStaticMesh _returnvalue_4 "/Game/Props/centerrock2.centerrock2")))))))
        (:1
          (Components|StaticMesh|SetStaticMesh _returnvalue_2 "/Game/Tiles/darkgrass.darkgrass")
          (goto _label))
        (:2
          (Components|StaticMesh|SetStaticMesh _returnvalue_2 "/Game/Tiles/highwayunmarked.highwayunmarked"))
        (:3
          (Components|StaticMesh|SetStaticMesh _returnvalue_2 "/Game/Tiles/railroad.railroad")
          (if (== _index (/ (Variables|Default|GetLaneLength) 2))
            (bind _returnvalue_5 (Game|SpawnActorfromClass "/Game/Blueprints/RR_Crossing.RR_Crossing_C" (Math|Transform|MakeTransform (Math|Vector|MakeVector (+ (.x (Variables|Default|GetSpawnVector)) 4e+01) (- (.y (Transformation|GetActorLocation)) 4e+01) 1e+01) "0, 0, 0" "1.000000,1.000000,1.000000") "Undefined" 0 0))
            (Variables|Default|SetRRCrossing _returnvalue_5)))))
    (else
      (switch int _output_get
        (:4
          (CallFunction|SpawnMarkedLane))
        (:5
          (CallFunction|SpawnWaterLane))))))

(fn SpawnMarkedLane
  (for _index (range 0 (Variables|Default|GetLaneLength))
    (bind _output_get (Variables|Default|SetSpawnVector (Math|Vector|MakeVector (Math|Conversions|ToFloat(Integer) (* _index 80)) 0.0 0.0)))
    (bind _returnvalue (AddComponent|AddStaticMeshComponent false (Math|Conversions|ToTransform(Vector) _output_get)))
    (Math|Integer|CompareInt (Math|Integer|%(Integer) _index 2)
      (:>
        (Components|StaticMesh|SetStaticMesh _returnvalue "/Game/Tiles/highwaymarked.highwaymarked"))
      (:==
        (Components|StaticMesh|SetStaticMesh _returnvalue "/Game/Tiles/highwayunmarked.highwayunmarked")))))

(fn SpawnWaterLane
  (bind _lanelength (Variables|Default|GetLaneLength))
  (bind _returnvalue (/ _lanelength 4))
  (Variables|Default|SetCarDir (Math|Random|RandomBool))
  (Variables|Default|SetSpawnLilyPads (Math|Random|RandomBool))
  (for _index (range 0 _lanelength)
    (bind _output_get (Variables|Default|SetSpawnVector (Math|Vector|MakeVector (Math|Conversions|ToFloat(Integer) (* _index 80)) 0.0 0.0)))
    (bind _returnvalue_2 (Game|SpawnActorfromClass "/Game/Blueprints/BP_Water.BP_Water_C" (Math|Transform|MakeTransform (Math|Vector|MakeVector (.x _output_get) (.y (Transformation|GetActorLocation)) 0.0) "0, 0, 0" "1.000000,1.000000,1.000000") "Undefined" 0 0))
    (Math|Integer|CompareInt _index _returnvalue
      (:>
        (Math|Integer|CompareInt _index (* _returnvalue 3)
          (:>
            (Default|SetType _returnvalue_2 1 :!label _label))
          (:==
            (Default|SetType _returnvalue_2 3))
          (:<
            (Default|SetType _returnvalue_2)
            (if (and (Variables|Default|GetSpawnLilyPads) (>= (Math|Random|RandomFloat) 0.7))
              (bind _returnvalue_3 (AddComponent|AddStaticMeshComponent false (Math|Transform|MakeTransform (Math|Vector|MakeVector (.x (Variables|Default|GetSpawnVector)) 0.0 1e+01) "0, 0, 0" "1.750000,1.750000,1.000000")))
              (Components|StaticMesh|SetStaticMesh _returnvalue_3 "/Game/Props/lilypad.lilypad")))))
      (:==
        (Default|SetType _returnvalue_2 2))
      (:<
        (goto _label)))))

(fn HighwayTick
  (if (<= (Variables|Default|GetTimer) 0.0)
    (Variables|Default|SetTimer (Math|Random|RandomFloatinRange 1.5 1e+01))
    (CallFunction|SpawnCar)
    (else
      (Variables|Default|SetTimer (- (Variables|Default|GetTimer) (Utilities|Time|GetWorldDeltaSeconds))))))

(fn SpawnCar
  (bind _returnvalue (Transformation|GetActorLocation))
  (bind _cardir (Variables|Default|GetCarDir))
  (switch int (Math|Random|RandomInteger 3)
    (:0
      (bind _returnvalue_2 (Game|SpawnActorfromClass "/Game/Blueprints/BP_Taxi.BP_Taxi_C" (Math|Transform|MakeTransform (Math|Vector|MakeVector 0.0 (.y _returnvalue) 1e+01) "0, 0, 0" "1.000000,1.000000,1.000000") "Undefined" 0 0))
      (if _cardir
        (bind _result (Math|Float|NegateFloat (Variables|/Game/Blueprints/BP_Taxi.BP_Taxi_C|GetSpeed _returnvalue_2))
          (:%20%20
            (Variables|/Game/Blueprints/BP_Taxi.BP_Taxi_C|SetSpeed _returnvalue_2 _result)
            (Transformation|AddActorWorldOffset _returnvalue_2 (Math|Vector|MakeVector 3.2e+03 0.0 0.0))
            (Class|Actor|AddActorWorldRotation _returnvalue_2 "0.000000,180.000000,0.000000")))))
    (:1
      (bind _returnvalue_3 (Game|SpawnActorfromClass "/Game/Blueprints/BP_Police.BP_Police_C" (Math|Transform|MakeTransform (Math|Vector|MakeVector 0.0 (.y _returnvalue) 1e+01) "0, 0, 0" "1.000000,1.000000,1.000000") "Undefined" 0 0))
      (if _cardir
        (bind _result_2 (Math|Float|NegateFloat (Variables|/Game/Blueprints/BP_Police.BP_Police_C|GetSpeed _returnvalue_3))
          (:%20%20
            (Variables|/Game/Blueprints/BP_Police.BP_Police_C|SetSpeed _returnvalue_3 _result_2)
            (Transformation|AddActorWorldOffset _returnvalue_3 (Math|Vector|MakeVector 3.2e+03 0.0 0.0))
            (Class|Actor|AddActorWorldRotation _returnvalue_3 "0.000000,180.000000,0.000000")))))
    (:2
      (bind _returnvalue_4 (Game|SpawnActorfromClass "/Game/Blueprints/BP_Fedex.BP_Fedex_C" (Math|Transform|MakeTransform (Math|Vector|MakeVector 0.0 (.y _returnvalue) 1e+01) "0, 0, 0" "1.000000,1.000000,1.000000") "Undefined" 0 0))
      (if _cardir
        (bind _result_3 (Math|Float|NegateFloat (Variables|/Game/Blueprints/BP_Fedex.BP_Fedex_C|GetSpeed _returnvalue_4))
          (:%20%20
            (Variables|/Game/Blueprints/BP_Fedex.BP_Fedex_C|SetSpeed _returnvalue_4 _result_3)
            (Transformation|AddActorWorldOffset _returnvalue_4 (Math|Vector|MakeVector 3.2e+03 0.0 0.0))
            (Class|Actor|AddActorWorldRotation _returnvalue_4 "0.000000,180.000000,0.000000")))))))

(fn HighwayStart
  (Variables|Default|SetTimer (Math|Random|RandomFloatinRange 0.75 4.0))
  (Variables|Default|SetCarDir (Math|Random|RandomBool)))

(fn Initialize
  (switch int (Variables|Default|GetLaneType)
    (:2
      (CallFunction|HighwayStart))
    (:4
      (CallFunction|HighwayStart))))

(fn SpawnTrain
  (Game|SpawnActorfromClass "/Game/Blueprints/BP_Train.BP_Train_C" (Math|Transform|MakeTransform (Math|Vector|MakeVector -2e+02 (.y (Transformation|GetActorLocation)) 0.0) "0, 0, 0" "1.000000,1.000000,1.000000") "Undefined" 0 0))

(fn RailroadTick
  (bind _rrcrossing (Variables|Default|GetRRCrossing))
  (if (<= (Variables|Default|GetTimer) 0.0)
    (Variables|Default|SetTimer (Math|Random|RandomFloatinRange 1e+01 2e+01))
    (CallFunction|SpawnTrain)
    (else
      (Variables|Default|SetTimer (- (Variables|Default|GetTimer) (Utilities|Time|GetWorldDeltaSeconds)))
      (if (<= (Variables|Default|GetTimer) 3.0)
        (Variables|/Game/Blueprints/RR_Crossing.RR_Crossing_C|Setactivated _rrcrossing true)
        (else
          (Default|DIsableLight _rrcrossing))))))

(fn WaterTick
  (if (not (Variables|Default|GetSpawnLilyPads))
    (if (<= (Variables|Default|GetTimer) 0.0)
      (Variables|Default|SetTimer (Math|Random|RandomFloatinRange 1.0 2.0))
      (bind _returnvalue (Game|SpawnActorfromClass "/Game/Blueprints/BP_Log.BP_Log_C" (Math|Transform|MakeTransform (Math|Vector|MakeVector 0.0 (.y (Transformation|GetActorLocation)) 0.0) "0, 0, 0" "1.000000,1.000000,1.000000") "Undefined" 0 0))
      (Default|SetSize _returnvalue (Math|Random|RandomInteger 4))
      (if (Variables|Default|GetCarDir)
        (Math|Float|NegateFloat (Variables|/Game/Blueprints/BP_Log.BP_Log_C|GetSpeed _returnvalue)
          (:%20%20
            (Transformation|AddActorWorldOffset _returnvalue (Math|Vector|MakeVector 3.2e+03 0.0 0.0)))))
      (else
        (Variables|Default|SetTimer (- (Variables|Default|GetTimer) (Utilities|Time|GetWorldDeltaSeconds)))))))