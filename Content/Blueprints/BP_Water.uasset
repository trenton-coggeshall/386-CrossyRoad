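; BP_Water is a water piece with a static mesh that sinks any pig that hits it.
; A hit on the mesh component casts the other actor to BP_Pig and calls its SinkPig function.
; SetType swaps the mesh between bright base, dark base, bright top and bright bottom variants based on an index.
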(event OnComponentHit(waterdarkBase)
  (params (HitComponent :type Primitive%20Component%20Object%20Reference) (OtherActor :type Actor%20Object%20Reference) (OtherComp :type Primitive%20Component%20Object%20Reference) (NormalImpulse :type Vector :default "0, 0, 0") (Hit :type Hit%20Result%20Structure%20%28by%20ref%29))
  (bind _asbp_pig (Utilities|Casting|CastToBP_Pig OtherActor))
  (Default|SinkPig _asbp_pig))

(event EventBeginPlay)

(event Collision|EventActorBeginOverlap
  (params (OtherActor :type Actor%20Object%20Reference)))

(event EventTick
  (params (DeltaSeconds :type Float%20%28single-precision%29)))

(fn ConstructionScript)

(fn SetType
  (params (type :type Integer))
  (switch int type
    (:0
      (Components|StaticMesh|SetStaticMesh (Variables|Default|GetwaterdarkBase) "/Game/Tiles/waterbrightBase.waterbrightBase"))
    (:1
      (Components|StaticMesh|SetStaticMesh (Variables|Default|GetwaterdarkBase) "/Game/Tiles/waterdarkBase.waterdarkBase"))
    (:2
      (Components|StaticMesh|SetStaticMesh (Variables|Default|GetwaterdarkBase) "/Game/Tiles/waterbrightTop.waterbrightTop"))
    (:3
      (Components|StaticMesh|SetStaticMesh (Variables|Default|GetwaterdarkBase) "/Game/Tiles/waterbrightBottom.waterbrightBottom"))))